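; SpawnVolume is an enemy spawner that runs endless waves of AI pawns inside its volume.
; After a preparation delay, BeginPlay loops timed spawns and pauses between waves; CurrentWave increments, but wave size stays fixed.
; Spawn rolls against cumulative percentage chances for Goliath, Wraith or Swarmer, placing it randomly within the scaled box extent and printing a debug message.
; Rolls above the combined chances spawn nothing, and the WaveNumber input is unused.
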(event EventBeginPlay
  ;[1 1 1] Spawn ennemies until spawnleft == 0
  (Variables|Default|SetCurrentWave 1)
  (Variables|Default|SetMaxSpawn 5)
  (Utilities|FlowControl|Delay (Variables|Default|GetpreparationTime))
  (Variables|Default|Setspawnleft (Variables|Default|GetMaxSpawn) :!label _label)
  (if (> (Variables|Default|Getspawnleft) 0) :!label _label_2
    (Utilities|FlowControl|Delay (Variables|Default|GetspawnDelay))
    (CallFunction|Spawn)
    (Variables|Default|Setspawnleft (- (Variables|Default|Getspawnleft) 1))
    (goto _label_2)
    (else
      ;[1 1 1] Delay before the next wave
      (Utilities|FlowControl|Delay (Variables|Default|GettimeBetweenWaves))
      (Variables|Default|SetCurrentWave (+ (Variables|Default|GetCurrentWave) 1))
      (goto _label))))

(fn ConstructionScript)

(fn Spawn
  (params (WaveNumber :type Integer))
  (bind _returnvalue (Transformation|GetActorLocation))
  (bind _spawnrotation (Variables|Default|GetspawnRotation))
  (bind _volume (Variables|Default|GetVolume))
  (bind _returnvalue_2 (Components|Box|GetScaledBoxExtent _volume))
  (bind (_x _y _z) (Math|Vector|BreakVector _returnvalue_2))
  (bind _returnvalue_3 (* _z -1.0))
  (bind _returnvalue_4 (* _x -1.0))
  (bind _returnvalue_5 (* _y -1.0))
  (bind _returnvalue_6 (Math|Random|RandomFloatinRange _returnvalue_3 _z))
  (bind _returnvalue_7 (Math|Random|RandomFloatinRange _returnvalue_4 _x))
  (bind _returnvalue_8 (Math|Random|RandomFloatinRange _returnvalue_5 _y))
  (bind _returnvalue_9 (Math|Vector|MakeVector _returnvalue_7 _returnvalue_8 _returnvalue_6))
  (bind _returnvalue_10 (+ _returnvalue_9 _returnvalue))
  (bind _returnvalue_11 (Math|Transform|MakeTransform _returnvalue_10 _spawnrotation))
  (bind (_location _rotation) (Math|Transform|BreakTransform _returnvalue_11))
  ;[1 1 1] Spawn chances for each enemy type
  (bind _output_get (Variables|Default|SetrandomTemp (Math|Random|RandomFloat)))
  (if (< _output_get (/ (Math|Conversions|ToFloat(Integer) (Variables|Default|GetbigChance)) 1e+02))
    (AI|SpawnAIFromClass "/Game/SliceDice/Blueprints/Enemies/Goliath.Goliath_C" 0 _location _rotation false)
    (Development|PrintString "HelloGoliath")
    (elif (< (Variables|Default|GetrandomTemp) (/ (Math|Conversions|ToFloat(Integer) (+ (Variables|Default|GetbigChance) (Variables|Default|GetRangedChance))) 1e+02))
      (AI|SpawnAIFromClass "/Game/SliceDice/Blueprints/Enemies/Wraith.Wraith_C" 0 _location _rotation false)
      (Development|PrintString "HelloWraith")
      (elif (< (Variables|Default|GetrandomTemp) (/ (Math|Conversions|ToFloat(Integer) (+ (Variables|Default|GetbigChance) (Variables|Default|GetRangedChance) (Variables|Default|GetSwarmerChance))) 1e+02))
        (AI|SpawnAIFromClass "/Game/SliceDice/Blueprints/Enemies/Swarmer.Swarmer_C" 0 _location _rotation false)
        (Development|PrintString "HelloSwarmer")))))