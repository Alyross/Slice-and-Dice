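; Base enemy Blueprint whose skeletal mesh and material are configurable per variant through the construction script, which applies a dynamic material instance.
; Incoming damage lowers health, briefly swapping to a hit-flash material, or spawns an explosion and destroys the actor when health runs out.
; Hitting a Character applies damage after a one-second delay if it passes a "Player" component tag check.
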(event EventBeginPlay)

(event EventActorBeginOverlap
  (params (OtherActor :type Actor%20Object%20Reference)))

(event EventTick
  (params (DeltaSeconds :type Float%20%28single-precision%29)))

(event EventAnyDamage
  (params (Damage :type Float%20%28single-precision%29) (DamageType :type Damage%20Type%20Object%20Reference) (InstigatedBy :type Controller%20Object%20Reference) (DamageCauser :type Actor%20Object%20Reference))
  ;[1 1 1] Take dmg and die
  (Variables|Default|SetHealth (- (Variables|Default|GetHealth) Damage))
  (if (<= (Variables|Default|GetHealth) 0.0)
    (Effects|SpawnEmitteratLocation "/Game/StarterContent/Particles/P_Explosion.P_Explosion" (Transformation|GetActorLocation))
    (Actor|DestroyActor)
    (else
      (Rendering|Material|SetMaterial 0 "/Game/StarterContent/Materials/_HitFlash._HitFlash")
      (Utilities|FlowControl|Delay 0.08)
      (Rendering|Material|SetMaterial 0 (Variables|Default|GetMeshMaterial)))))

(event EventHit
  (params (MyComp :type Primitive%20Component%20Object%20Reference) (Other :type Actor%20Object%20Reference) (OtherComp :type Primitive%20Component%20Object%20Reference) (bSelfMoved :type Boolean) (HitLocation :type Vector :default "0, 0, 0") (HitNormal :type Vector :default "0, 0, 0") (NormalImpulse :type Vector :default "0, 0, 0") (Hit :type Hit%20Result%20Structure%20%28by%20ref%29))
  ;[1 1 1] Apply dmg to player
  (bind _ascharacter (Utilities|Casting|CastToCharacter Other))
  (Utilities|FlowControl|Delay 1.0)
  (if (Components|ComponentHasTag _ascharacter "Player")
    (Game|Damage|ApplyDamage Other (Variables|Default|GetDamage) 0 self)))

(fn ConstructionScript
  ;[1 1 1] Base class for enemy, this script sets lets you set up different meshes and materials for all different enemies linked to this BP
  (if (not (== (Variables|Default|GetvariableMesh) 0))
    (Class|SkinnedMeshComponent|SetSkeletalMesh (Variables|Default|GetvariableMesh))
    (bind _returnvalue (Rendering|Material|CreateDynamicMaterialInstance (Variables|Default|GetMeshMaterial) :!class /Script/Engine.KismetMaterialLibrary))
    (Rendering|Material|SetMaterial 0 _returnvalue)))